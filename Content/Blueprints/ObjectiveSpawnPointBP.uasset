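; Objective spawn point that displays an objective and hands it to a train car that overlaps it.
; The mesh stays hidden until the OnObjectiveSet event fires, then shows with a material indexed by the objective type.
; When a TrainCar overlaps while the spawn data is active, the point passes the objective type to the car, clears its data and hides the mesh again.
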(event `self.ReceiveBeginPlay`
  (`SceneComponent.SetVisibility` (`self.StaticMesh`) false true)
  (add `self.OnObjectiveSet` (delegate `OnObjectiveSet_Event_0`)))

(event `OnObjectiveSet_Event_0`
  (bind _staticmesh (`self.StaticMesh`))
  (`PrimitiveComponent.SetMaterial` _staticmesh 0 (`|GetArrayItem` (`self.MaterialInstaRef`) (`KismetMathLibrary.Conv_ByteToInt` (`.ObjectiveType` (break `ObjectiveState` (`self.SpawnData`))))))
  (`SceneComponent.SetVisibility` _staticmesh true true))

(event `self.ReceiveActorBeginOverlap`
  (params (OtherActor :type "Actor Object Reference"))
  (bind (_bactive _objectivetype) (break `ObjectiveState` (`self.SpawnData`)))
  (bind _astrain_car (cast `TrainCar` OtherActor))
  (if _bactive
    (`TrainCar.SetCarryObjective` _astrain_car _objectivetype)
    (set `self.SpawnData` (struct))
    (`SceneComponent.SetVisibility` (`self.StaticMesh`) false true)))

(fn `UserConstructionScript`)