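; Track actor that builds a deformed mesh track along its spline, entirely in the Construction Script.
; It divides the spline into fixed-length steps and adds an X-forward spline mesh component for each, including a final one at the spline's end.
; Each segment takes local-space positions and unscaled tangents sampled by distance at both of its ends.
; The event graph holds only disabled placeholder events.
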(fn `UserConstructionScript`
  (for _index (range (+ (`KismetMathLibrary.FTrunc` (/ (`SplineComponent.GetSplineLength` (`self.Spline`)) 100.0)) 1))
    (bind _returnvalue (`AddComponent|NODE_AddSplineMeshComponent-0`))
    (`SplineMeshComponent.SetForwardAxis` _returnvalue "X" true)
    (bind _returnvalue_2 (* _index 100.0))
    (bind _returnvalue_3 (* (+ _index 1) 100.0))
    (`SplineMeshComponent.SetStartAndEnd` _returnvalue (`SplineComponent.GetLocationAtDistanceAlongSpline` (`self.Spline`) _returnvalue_2 "Local") (`SplineComponent.GetTangentAtDistanceAlongSpline` (`self.Spline`) _returnvalue_2 "Local") (`SplineComponent.GetLocationAtDistanceAlongSpline` (`self.Spline`) _returnvalue_3 "Local") (`SplineComponent.GetTangentAtDistanceAlongSpline` (`self.Spline`) _returnvalue_3 "Local") true)))