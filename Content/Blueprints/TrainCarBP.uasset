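; Train car Blueprint that shows its objective state by swapping materials on its two static meshes.
; On BeginPlay it binds to the OnRefreshTrainState dispatcher.
; On each refresh, an active objective selects a material from MaterialRef, indexed by its objective type, while an inactive one restores TrainDefault through DefaultMaterialApply.
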(event `self.ReceiveBeginPlay`
  (add `self.OnRefreshTrainState` (delegate `OnRefreshTrainState_Event_0`)))

(event `OnRefreshTrainState_Event_0`
  (bind (_bactive _objectivetype) (break `ObjectiveState` (`self.ObjectiveState`)))
  (bind _output (`|GetArrayItem` (`self.MaterialRef`) (`KismetMathLibrary.Conv_ByteToInt` _objectivetype)))
  (if _bactive
    (`PrimitiveComponent.SetMaterial` (`self.StaticMesh`) 0 _output)
    (`PrimitiveComponent.SetMaterial` (`self.StaticMesh1`) 0 _output)
    (else
      (`self.DefaultMaterialApply`))))

(fn `DefaultMaterialApply`
  (`PrimitiveComponent.SetMaterial` (`self.StaticMesh`) 0 "/Game/Materials/TrainDefault.TrainDefault")
  (`PrimitiveComponent.SetMaterial` (`self.StaticMesh1`) 0 "/Game/Materials/TrainDefault.TrainDefault"))

(fn `UserConstructionScript`)