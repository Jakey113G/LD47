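; Track switch actor that responds to train cars entering it and can be toggled active by keyboard input.
; Holding the 1 key sets the switch active and shows its Arrow component; releasing it deactivates the switch and hides the arrow.
; Begin-overlap events cast to TrainCar and pass matching actors to OnActorEnteringSwitch, whose logic lives outside these graphs.
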(event `Key|One`
  (params (Key :type "Key Structure"))
  (:`Pressed`
    (`self.ActiveSwitch`))
  (:`Released`
    (`self.DeactivateSwitch`)))

(event `self.ReceiveActorBeginOverlap`
  (params (OtherActor :type "Actor Object Reference"))
  (bind _astrain_car (cast `TrainCar` OtherActor))
  (`self.OnActorEnteringSwitch` _astrain_car))

(fn `ActiveSwitch`
  (`self.SetIsSwitchActive` true)
  (`SceneComponent.SetVisibility` (`self.Arrow`) true false))

(fn `DeactivateSwitch`
  (`self.SetIsSwitchActive` false)
  (`SceneComponent.SetVisibility` (`self.Arrow`) false false))

(fn `UserConstructionScript`)